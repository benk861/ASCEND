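; BP_LaserCube is a laser cube for the FPS puzzle game that supplies an outgoing beam segment from its Arrow component.
; GetReflectionVector returns a start at the arrow's world location and an end along its forward vector, MaxNonReflectDistantion away, so the direction follows the arrow rather than an incoming angle.
; Tick, Hit and the construction script only call the parent class.
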(event `self.ReceiveTick`
  (params (DeltaSeconds :type "Float (single-precision)"))
  ;[1 1 1] Physics root
  (`parent.ReceiveTick` DeltaSeconds))

(event `self.ReceiveHit`
  (params (MyComp :type "PrimitiveComponent Object Reference") (Other :type "Actor Object Reference") (OtherComp :type "PrimitiveComponent Object Reference") (bSelfMoved :type Boolean) (HitLocation :type "Vector Structure") (HitNormal :type "Vector Structure") (NormalImpulse :type "Vector Structure") (Hit :type "HitResult Structure (by ref)"))
  ;[1 1 1] Physics root
  (`parent.ReceiveHit` MyComp Other OtherComp bSelfMoved HitLocation HitNormal NormalImpulse Hit))

(fn `getReflectionVector`
  (returns (Start :type "Vector Structure") (End :type "Vector Structure"))
  (bind _arrow (`self.Arrow`))
  (bind _returnvalue (`SceneComponent.K2_GetComponentLocation` _arrow))
  (return _returnvalue (+ _returnvalue (* (`SceneComponent.GetForwardVector` _arrow) (`self.MaxNonReflectDistantion`)))))

(fn `UserConstructionScript`
  (`parent.UserConstructionScript`))