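; Main menu actor that shows a menu in a widget component and moves the player's view between linked menu actors.
; On BeginPlay it plays the menu music and, if the widget is a W_MainMenu, binds to its transition event.
; A valid index from that event selects a linked menu, moves collision from this actor to that one, and eases the view target over to it.
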(event `self.ReceiveBeginPlay`
  ;[1 1 1] Transition to other menu
  (`GameplayStatics.PlaySound2D` "/Game/MainContent/Audio/Music/MainMenu/MainMenuMusicSoundCue.MainMenuMusicSoundCue" 1.0 1.0 0.0 null null false)
  (bind _asmain_menu (cast `/Game/MainContent/UI/W_MainMenu` (`WidgetComponent.GetUserWidgetObject` (`self.Widget`))))
  (add `/Game/MainContent/UI/W_MainMenu.TransitionToLinkedMenu` _asmain_menu (delegate `OnTransitionBetweenMenus`)))

(event `OnTransitionBetweenMenus`
  (params (MenuIndex :type Integer))
  ;[1 1 1] Transition to other menu
  (if (`KismetArrayLibrary.Array_IsValidIndex` (`|MakeArray` (`self.LinkedMenus`)) MenuIndex)
    (`self.TransitionTo` (`|GetArrayItem` (`|MakeArray` (`self.LinkedMenus`)) MenuIndex))))

(event `TransitionTo`
  (params (`New Menu` :type "/Game/MainContent/Levels/MainMenu/BP_Menu Object Reference"))
  (`self.SetActorEnableCollision` false)
  (`self.SetActorEnableCollision` `New Menu` true)
  (`PlayerController.SetViewTargetWithBlend` (`GameplayStatics.GetPlayerController` 0) `New Menu` 5.0 "VTBlend_EaseInOut" 5.0 false))

(fn `UserConstructionScript`)