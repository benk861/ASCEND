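; Ladder actor that switches the first-person character into and out of climbing through overlap volumes.
; Entering the main Box with the capsule passes the ladder's forward vector to the character and blocks ToOut1 exits for 0.2 seconds.
; Leaving the Box ends climbing, adding an exit boost if the character overlaps ToOut.
; Overlapping ToOut1 also ends climbing once that short lockout expires.
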(event `self.Box.OnComponentBeginOverlap`
  (params (OverlappedComponent :type "PrimitiveComponent Object Reference") (OtherActor :type "Actor Object Reference") (OtherComp :type "PrimitiveComponent Object Reference") (OtherBodyIndex :type Integer) (bFromSweep :type Boolean) (SweepResult :type "HitResult Structure (by ref)"))
  (bind _ascapsule_collision (cast `CapsuleComponent` OtherComp))
  (bind _asbp_first_person_character (cast `/Game/MainContent/Blueprints/Character/BP_FirstPersonCharacter` (`ActorComponent.GetOwner` _ascapsule_collision)))
  (`/Game/MainContent/Blueprints/Character/BP_FirstPersonCharacter.EnteredLadder` _asbp_first_person_character (`self.GetActorForwardVector`))
  (set `self.CanOut` false)
  (`KismetSystemLibrary.Delay` 0.2)
  (set `self.CanOut` true))

(event `self.Box.OnComponentEndOverlap`
  (params (OverlappedComponent :type "PrimitiveComponent Object Reference") (OtherActor :type "Actor Object Reference") (OtherComp :type "PrimitiveComponent Object Reference") (OtherBodyIndex :type Integer))
  (bind _ascapsule_collision (cast `CapsuleComponent` OtherComp))
  (bind _asbp_first_person_character (cast `/Game/MainContent/Blueprints/Character/BP_FirstPersonCharacter` (`ActorComponent.GetOwner` _ascapsule_collision)))
  (if (`PrimitiveComponent.IsOverlappingActor` (`self.ToOut`) _asbp_first_person_character)
    (`/Game/MainContent/Blueprints/Character/BP_FirstPersonCharacter.ExitBoost` _asbp_first_person_character))
  (`/Game/MainContent/Blueprints/Character/BP_FirstPersonCharacter.ExittedLadder` _asbp_first_person_character))

(event `self.ToOut1.OnComponentBeginOverlap`
  (params (OverlappedComponent :type "PrimitiveComponent Object Reference") (OtherActor :type "Actor Object Reference") (OtherComp :type "PrimitiveComponent Object Reference") (OtherBodyIndex :type Integer) (bFromSweep :type Boolean) (SweepResult :type "HitResult Structure (by ref)"))
  (if (`self.CanOut`)
    (bind _ascapsule_collision (cast `CapsuleComponent` OtherComp))
    (bind _asbp_first_person_character (cast `/Game/MainContent/Blueprints/Character/BP_FirstPersonCharacter` (`ActorComponent.GetOwner` _ascapsule_collision)))
    (`/Game/MainContent/Blueprints/Character/BP_FirstPersonCharacter.ExittedLadder` _asbp_first_person_character)))

(fn `UserConstructionScript`)