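; Double-jump ability actor, marked OLD, that turns to face the player, with no jump logic in this graph.
; From BeginPlay, a self-calling Delay loop polls player distance until in range, then hands off to FacePlayer.
; FacePlayer repeatedly updates yaw toward the player without rechecking distance, so it keeps tracking once triggered.
; JumpOverlappedPlayer stores overlap state in CanJump, but the Tick branch reading it is empty.
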(event `self.ReceiveTick`
  (params (DeltaSeconds :type "Float (single-precision)"))
  (if (`self.CanJump`)
    _))

(event `self.ReceiveBeginPlay`
  (bind _asbp_first_person_character (cast `/Game/MainContent/Blueprints/Character/BP_FirstPersonCharacter` (`GameplayStatics.GetPlayerCharacter` 0)))
  (set `self.FirstPersonCharacterReference` _asbp_first_person_character)
  (`self.Should Rotate Event`))

(event `Face Player`
  (bind (_returnvalue_roll _returnvalue_pitch _returnvalue_yaw) (`KismetMathLibrary.BreakRotator` (`KismetMathLibrary.RInterpTo` (`self.K2_GetActorRotation`) (`KismetMathLibrary.FindLookAtRotation` (`self.K2_GetActorLocation`) (`self.K2_GetActorLocation` (`GameplayStatics.GetPlayerCharacter` 0))) (`GameplayStatics.GetWorldDeltaSeconds`))))
  (if (`self.Should Rotate?`)
    (`self.K2_SetActorRotation` (`KismetMathLibrary.MakeRotator` 0.0 0.0 _returnvalue_yaw))
    (`KismetSystemLibrary.Delay` 0.001)
    (`self.Face Player`)
    (else
      (`self.Should Rotate Event`))))

(event `Should Rotate Event`
  (if (<= (`self.GetDistanceTo` (`GameplayStatics.GetPlayerCharacter` 0)) 500.0)
    (set `self.Should Rotate?` true)
    (`self.Face Player`)
    (else
      (set `self.Should Rotate?` false)
      (`KismetSystemLibrary.Delay` 0.001)
      (`self.Should Rotate Event`))))

(fn `JumpOverlappedPlayer`
  (params (BeginOverlap :type Boolean))
  (set `self.CanJump` BeginOverlap))

(fn `UserConstructionScript`)