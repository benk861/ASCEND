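; BP_Mine is a mine actor for the mine ability that blasts the player character away when detonated.
; When its Sphere hits something, it zeroes velocity and stops simulating physics, so it stays where it lands.
; Explode launches the player, if inside the Explosion overlap, away from the Sphere toward a raised target point, at full force up close and inverse-distance falloff farther out, and returns the overlap result.
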(event `self.Sphere.OnComponentHit`
  (params (HitComponent :type "PrimitiveComponent Object Reference") (OtherActor :type "Actor Object Reference") (OtherComp :type "PrimitiveComponent Object Reference") (NormalImpulse :type "Vector Structure") (Hit :type "HitResult Structure (by ref)"))
  (bind _sphere (`self.Sphere`))
  (`/Engine/EditorBlueprintResources/StandardMacros.IsValid` _sphere
    (:`Is Valid`
      (`PrimitiveComponent.SetAllPhysicsLinearVelocity` _sphere (0.0 0.0 0.0) false)
      (`PrimitiveComponent.SetSimulatePhysics` _sphere false))))

(fn `Explode`
  (returns (Exploded :type Boolean))
  (bind _returnvalue (`GameplayStatics.GetPlayerCharacter` 0))
  (bind _returnvalue_2 (`SceneComponent.K2_GetComponentLocation` (`self.Sphere`)))
  (bind _returnvalue_3 (`PrimitiveComponent.IsOverlappingActor` (`self.Explosion`) _returnvalue))
  (bind _returnvalue_4 (* (`self.Direction`) 2500.0))
  (bind _returnvalue_5 (+ (`self.K2_GetActorLocation` _returnvalue) (0.0 0.0 100.0)))
  (if _returnvalue_3
    (set `self.Direction` (`KismetMathLibrary.Normal` (- _returnvalue_5 _returnvalue_2)))
    (bind _output_get (set `self.Distance` (`KismetMathLibrary.Vector_Distance` _returnvalue_5 _returnvalue_2)))
    (`/Engine/EditorBlueprintResources/StandardMacros.IncrementFloat` _output_get
      (:`  `
        (if (< (`self.Distance`) 370.0)
          (set `self.Force` _returnvalue_4)
          (else
            (set `self.Force` (/ _returnvalue_4 (/ (`self.Distance`) 400.0)))))
        (`Character.LaunchCharacter` _returnvalue (`self.Force`) true true)
        (return _returnvalue_3)))
    (else
      (return _returnvalue_3))))

(fn `UserConstructionScript`)