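; Grapple ability that pulls the player toward a BP_GrappleTarget and launches them on release.
; CanActivateAbility sphere-traces around the player and picks the target with a visible mesh closest to the camera's forward direction.
; First use switches to Flying, ignores move input and applies pulling force on a looping timer.
; Reuse or overlapping the target's sphere flips to release, restoring Walking with an upward-biased impulse, stronger on arrival.
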(event `CalculateForce`
  (set `self.GrappleForce` (* (`KismetMathLibrary.Normal` (- (`self.K2_GetActorLocation` (`self.Target`)) (`self.K2_GetActorLocation` (`GameplayStatics.GetPlayerCharacter` 0)))) 20000.0)))

(event `GrappleFirst`
  (bind _charactermovement (`Character.CharacterMovement` (`GameplayStatics.GetPlayerCharacter` 0)))
  (set `self.Multiplier` 120000.0)
  (`CharacterMovementComponent.SetMovementMode` _charactermovement "MOVE_Flying" 0)
  (set `MovementComponent.Velocity` (0.0 0.0 0.0) _charactermovement)
  (set `self.SecondUse` true)
  (`Controller.SetIgnoreMoveInput` (`GameplayStatics.GetPlayerController` 0) true)
  (set `self.SphereColl` (`self.GetComponentByClass` (`self.Target`) "/Script/Engine.SphereComponent"))
  (bind _returnvalue (`KismetSystemLibrary.K2_SetTimerDelegate` (delegate `Dragging`) 0.001 true)))

(event `GrappleSecond`
  (bind _charactermovement (`Character.CharacterMovement` (`GameplayStatics.GetPlayerCharacter` 0)))
  (set `self.SecondUse` false)
  (`Controller.SetIgnoreMoveInput` (`GameplayStatics.GetPlayerController` 0) false)
  (`KismetSystemLibrary.K2_ClearAndInvalidateTimerHandle` (stale `GrappleFirst` _returnvalue))
  (`CharacterMovementComponent.SetMovementMode` _charactermovement "MOVE_Walking" 0)
  (`CharacterMovementComponent.AddImpulse` _charactermovement (* (+ (`KismetMathLibrary.Normal` (`MovementComponent.Velocity` _charactermovement)) (0.0 0.0 0.6)) (`self.Multiplier`)) false))

(event `Dragging`
  (`self.CalculateForce`)
  (`CharacterMovementComponent.AddForce` (`Character.CharacterMovement` (`GameplayStatics.GetPlayerCharacter` 0)) (`self.GrappleForce`))
  (if (`PrimitiveComponent.IsOverlappingActor` (`self.SphereColl`) (`GameplayStatics.GetPlayerCharacter` 0))
    (set `self.Multiplier` (* (`self.Multiplier`) 1.45))
    (`/Engine/EditorBlueprintResources/StandardMacros.FlipFlop` :!label _label
      (:`A`
        (`self.GrappleFirst`))
      (:`B`
        (`self.GrappleSecond`)))))

(event `self.UseAbility`
  (goto _label))

(fn `CanActivateAbility`
  (returns (ReturnValue :type Boolean))
  (bind _returnvalue (`self.K2_GetActorLocation` (`GameplayStatics.GetPlayerCharacter` 0)))
  (if (`self.SecondUse`)
    (return true)
    (else
      (set `self.Target` null)
      (bind _outhits (`KismetSystemLibrary.SphereTraceMultiForObjects` _returnvalue _returnvalue 7000.0 (`|MakeArray` "ObjectTypeQuery7" :!type "EObjectTypeQuery Enum")))
      (set `self.PossibleTargets` _outhits)
      (set `self.Diffrence` 99999.0)
      (set `self.PlayerLooking` (`self.GetActorForwardVector` (`GameplayStatics.GetPlayerCameraManager` 0)))
      (for _array_element (`self.PossibleTargets`)
        (if (`SceneComponent.IsVisible` (`self.GetComponentByClass` (`.HitActor` (`GameplayStatics.BreakHitResult` _array_element)) "/Script/Engine.StaticMeshComponent"))
          (bind _returnvalue_2 (`KismetMathLibrary.Vector_Distance` (`KismetMathLibrary.Normal` (- (`self.K2_GetActorLocation` (`.HitActor` (`GameplayStatics.BreakHitResult` _array_element))) (`self.K2_GetActorLocation` (`GameplayStatics.GetPlayerCharacter` 0)))) (`self.PlayerLooking`)))
          (if (< _returnvalue_2 (`self.Diffrence`))
            (set `self.Diffrence` _returnvalue_2)
            (bind _asbp_grapple_target (cast `/Game/MainContent/Blueprints/Abilities/BP_GrappleTarget` (`.HitActor` (`GameplayStatics.BreakHitResult` _array_element))))
            (set `self.Target` _asbp_grapple_target))))
      (return (!= (`self.Target`) null)))))

(fn `UserConstructionScript`)