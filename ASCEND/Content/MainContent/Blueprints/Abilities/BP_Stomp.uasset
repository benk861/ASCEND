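; BP_Stomp is a player ability that slams the character downward out of the air.
; It can only activate while the Ascend player's movement component reports falling.
; On use it calls the parent ability, then launches the player with a strong downward velocity that overrides existing XY and Z motion.
; It then looks up the first-person character by class and adds a Niagara effect component if that character is not moving on the ground.
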(event `self.UseAbility`
  (`parent.UseAbility`)
  (`Character.LaunchCharacter` (`self.GetAscendPlayer`) (0.0 0.0 -2500.0) true true)
  (bind _returnvalue (`GameplayStatics.GetActorOfClass` "/Game/MainContent/Blueprints/Character/BP_FirstPersonCharacter.BP_FirstPersonCharacter_C"))
  (bind _asbp_first_person_character (cast `/Game/MainContent/Blueprints/Character/BP_FirstPersonCharacter` _returnvalue))
  (if (not (`NavMovementComponent.IsMovingOnGround` (`Character.CharacterMovement` _asbp_first_person_character)))
    (`AddComponent|NODE_AddNiagaraComponent-0`)))

(fn `CanActivateAbility`
  (returns (ReturnValue :type Boolean))
  (return (`NavMovementComponent.IsFalling` (`Character.CharacterMovement` (`self.GetAscendPlayer`)))))

(fn `UserConstructionScript`)