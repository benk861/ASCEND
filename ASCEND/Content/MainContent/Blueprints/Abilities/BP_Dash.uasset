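; BP_Dash is a player ability that dashes the character forward.
; On use it calls the parent ability logic, plays a dash sound and launches the Ascend player along its forward vector.
; The launch is weaker while the character is falling than on the ground, and it adds to current velocity rather than overriding it.
; The ability always reports that it can activate.
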(event `self.UseAbility`
  (bind _returnvalue (`self.GetAscendPlayer`))
  (bind _returnvalue_2 (`self.GetAscendPlayer`))
  (`parent.UseAbility`)
  (`GameplayStatics.PlaySound2D` "/Game/MainContent/Audio/Abilities/SFX_Dash.SFX_Dash" 1.0 1.0 0.0 null null false)
  (if (`NavMovementComponent.IsFalling` (`Pawn.GetMovementComponent` (`self.GetAscendPlayer`)))
    (`Character.LaunchCharacter` _returnvalue_2 (* (`self.GetActorForwardVector` _returnvalue_2) 3000.0) false false)
    (else
      (`Character.LaunchCharacter` _returnvalue (* (`self.GetActorForwardVector` _returnvalue) 10000.0) false false))))

(fn `CanActivateAbility`
  (returns (ReturnValue :type Boolean))
  (return true))

(fn `UserConstructionScript`)