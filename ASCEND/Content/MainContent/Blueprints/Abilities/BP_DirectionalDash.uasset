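; BP_DirectionalDash is an ability Blueprint that launches the first-person player along their look direction.
; Overlapping the actor caches the player character; using the ability then triggers the player's blur effect and a dash sound.
; The launch follows the control rotation's forward vector, vertical aim included, and overrides existing velocity, with slightly less force while falling.
; Activation is always allowed, as this Blueprint adds no conditions.
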(event `self.ReceiveActorBeginOverlap`
  (params (OtherActor :type "Actor Object Reference"))
  (`parent.ReceiveActorBeginOverlap` null)
  (bind _asbp_first_person_character (cast `/Game/MainContent/Blueprints/Character/BP_FirstPersonCharacter` (`self.GetAscendPlayer`)))
  (set `self.Player` _asbp_first_person_character))

(event `self.UseAbility`
  (`parent.UseAbility`)
  (`/Game/MainContent/Blueprints/Character/BP_FirstPersonCharacter.Blur` (`self.Player`))
  (`GameplayStatics.PlaySound2D` "/Game/MainContent/Audio/Abilities/SFX_Dash.SFX_Dash" 1.0 1.0 0.0 null null false)
  (if (`NavMovementComponent.IsFalling` (`Pawn.GetMovementComponent` (`self.Player`)))
    (set `self.LaunchForce` 2500.0)
    (else
      (set `self.LaunchForce` 2750.0)))
  (bind _dashdirection (`self.CalculateDashDirection` (`self.LaunchForce`)))
  (`Character.LaunchCharacter` (`self.Player`) _dashdirection true true))

(fn `CalculateDashDirection`
  (params (LaunchForce :type "Float (double-precision)"))
  (returns (DashDirection :type "Vector Structure"))
  (return (* (`KismetMathLibrary.Conv_RotatorToVector` (`Pawn.GetControlRotation` (`self.GetAscendPlayer`))) LaunchForce)))

(fn `CanActivateAbility`
  (returns (ReturnValue :type Boolean))
  (return true))

(fn `UserConstructionScript`)