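; BP_Stomp is a player ability that slams an airborne character toward the ground.
; It can activate only while the player's movement component reports falling.
; On use it runs the parent ability logic, flags the first-person character as stomping, then launches it sharply downward with velocity overridden on all axes and posts an in-air Wwise sound.
; Landing and impact are not handled in this Blueprint.
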(event `self.UseAbility`
  (`parent.UseAbility`)
  (bind _asbp_first_person_character (cast `/Game/MainContent/Blueprints/Character/BP_FirstPersonCharacter` (`self.GetAscendPlayer`)))
  (set `/Game/MainContent/Blueprints/Character/BP_FirstPersonCharacter.IsStomping` true _asbp_first_person_character)
  (`Character.LaunchCharacter` (`self.GetAscendPlayer`) (0.0 0.0 -2500.0) true true)
  (`AkGameplayStatics.PostEvent` "/Game/MainContent/Blueprints/Abilities/Stomp/Stomp_InAir.Stomp_InAir"))

(fn `CanActivateAbility`
  (returns (ReturnValue :type Boolean))
  (return (`NavMovementComponent.IsFalling` (`Character.CharacterMovement` (`self.GetAscendPlayer`)))))

(fn `UserConstructionScript`)