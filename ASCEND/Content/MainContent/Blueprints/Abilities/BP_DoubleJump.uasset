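; Double jump ability Blueprint for the Ascend player, allowed only while the player's CanDoubleJump flag is set.
; When used mid-fall, it runs the parent ability logic, plays a sound and launches the character upward, overriding Z velocity with the movement component's jump velocity plus a fixed boost.
; That air jump then clears the flag.
; When the player is not falling, it performs a normal jump instead, skipping the parent logic.
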(event `self.UseAbility`
  (bind _returnvalue (`self.GetAscendPlayer`))
  (if (`NavMovementComponent.IsFalling` (`Character.CharacterMovement` _returnvalue))
    (`parent.UseAbility`)
    (`GameplayStatics.PlaySound2D` "/Game/MainContent/Audio/Abilities/SFX_DoubleJump.SFX_DoubleJump" 1.0 1.0 0.0 null null)
    (`Character.LaunchCharacter` (`self.GetAscendPlayer`) (`KismetMathLibrary.MakeVector` 0.0 0.0 (+ (`CharacterMovementComponent.JumpZVelocity` (cast `CharacterMovementComponent` (`Pawn.GetMovementComponent` (`self.GetAscendPlayer`)) :!pure true)) 250.0)) false true)
    (set `PlayerCharacter.bCanDoubleJump` false (`self.GetAscendPlayer`))
    (else
      (`Character.Jump` _returnvalue))))

(fn `CanActivateAbility`
  (returns (ReturnValue :type Boolean))
  (return (`PlayerCharacter.bCanDoubleJump` (`self.GetAscendPlayer`))))

(fn `UserConstructionScript`)