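; Player ability that throws a mine and detonates it on a second use.
; The first use spawns BP_Mine ahead of player 0, launches it along the aim direction and schedules its removal after TimeToDestroy.
; The next use calls Explode on the live mine, destroying it on success or refunding a charge on failure.
; BeginPlay doubles max charges and also raises the charges left, as both throw and detonation go through the parent UseAbility.
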(event `self.ReceiveBeginPlay`
  (bind _returnvalue (* (`self.GetMaxCharges`) 2))
  (`self.SetMaxCharges` _returnvalue)
  (`self.SetChargesLeft` _returnvalue))

(event `self.UseAbility`
  (bind _returnvalue (`GameplayStatics.GetPlayerCharacter` 0))
  (`parent.UseAbility`)
  (if (not (`self.Deployed`))
    (bind _returnvalue_2 (`|SpawnActorFromClass` "/Game/MainContent/Blueprints/Abilities/BP_Mine.BP_Mine_C" (`KismetMathLibrary.Conv_VectorToTransform` (+ (`self.K2_GetActorLocation` _returnvalue) (* (`self.GetActorForwardVector` _returnvalue) 100.0))) "AdjustIfPossibleButAlwaysSpawn" "OverrideRootScale" null null))
    (`PrimitiveComponent.AddImpulse` (`/Game/MainContent/Blueprints/Abilities/BP_Mine.Sphere` _returnvalue_2) (* (`KismetMathLibrary.Conv_RotatorToVector` (`Pawn.GetControlRotation` _returnvalue)) 1800.0) "None" true)
    (set `self.Deployed` true)
    (`KismetSystemLibrary.Delay` (`self.TimeToDestroy`))
    (`/Engine/EditorBlueprintResources/StandardMacros.IsValid` _returnvalue_2
      (:`Is Valid`
        (`self.K2_DestroyActor` _returnvalue_2)
        (set `self.Deployed` false)))
    (else
      (`/Engine/EditorBlueprintResources/StandardMacros.IsValid` _returnvalue_2
        (:`Is Valid`
          (bind _exploded (`/Game/MainContent/Blueprints/Abilities/BP_Mine.Explode` _returnvalue_2))
          (if _exploded
            (`self.K2_DestroyActor` _returnvalue_2)
            (set `self.Deployed` false)
            (else
              (`self.SetChargesLeft` (+ (`self.ChargesLeft`) 1)))))))))

(fn `UserConstructionScript`)