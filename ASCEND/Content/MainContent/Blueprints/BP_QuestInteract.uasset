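; BP_QuestInteract is a quest interaction Blueprint that shows a text prompt only while the player is looking at it.
; Each Tick drives the Text component's visibility from IsPlayerLookingAt, which this Blueprint reads but never sets.
; While visible, the text billboards toward the player camera on yaw only, staying upright with zero pitch and roll.
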(event `self.ReceiveTick`
  (params (DeltaSeconds :type "Float (single-precision)"))
  (bind _bisplayerlookingat (`self.bIsPlayerLookingAt`))
  (bind (_returnvalue_roll _returnvalue_pitch _returnvalue_yaw) (`KismetMathLibrary.BreakRotator` (`KismetMathLibrary.FindLookAtRotation` (`PlayerCameraManager.GetCameraLocation` (`GameplayStatics.GetPlayerCameraManager` 0)) (`SceneComponent.K2_GetComponentLocation` (`self.Text`)))))
  (`SceneComponent.SetVisibility` (`self.Text`) _bisplayerlookingat false)
  (if _bisplayerlookingat
    (`SceneComponent.K2_SetWorldRotation` (`self.Text`) (`KismetMathLibrary.MakeRotator` 0.0 0.0 (+ _returnvalue_yaw 180.0)) false false)))

(fn `UserConstructionScript`)