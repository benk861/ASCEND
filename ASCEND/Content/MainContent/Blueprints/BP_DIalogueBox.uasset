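; BP_DIalogueBox is a one-shot trigger actor that starts a dialogue when BP_FirstPersonCharacter overlaps it.
; On overlap it disables the character's movement, adds a W_Dialogue widget to the viewport and switches input to UI only.
; It copies its own portraits, names, Talker and Messages into the widget, calls Click to begin, then destroys itself.
; Restoring movement and input is not handled here.
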(event `self.ReceiveActorBeginOverlap`
  (params (OtherActor :type "Actor Object Reference"))
  (bind _asbp_first_person_character (cast `/Game/MainContent/Blueprints/Character/BP_FirstPersonCharacter` OtherActor))
  (`CharacterMovementComponent.DisableMovement` (`Character.CharacterMovement` _asbp_first_person_character))
  (bind _returnvalue (`|CreateWidget` "/Game/MainContent/UI/W_Dialogue.W_Dialogue_C"))
  (bind _output_get (set `self.DialWidget` _returnvalue))
  (`UserWidget.AddToViewport` _output_get 0)
  (`WidgetBlueprintLibrary.SetInputMode_UIOnlyEx` (`GameplayStatics.GetPlayerController` 0) (`self.DialWidget`))
  (`Image.SetBrushFromTexture` (`/Game/MainContent/UI/W_Dialogue.First` (`self.DialWidget`)) (`self.First`) false)
  (`Image.SetBrushFromTexture` (`/Game/MainContent/UI/W_Dialogue.Second` (`self.DialWidget`)) (`self.Second`) false)
  (set `/Game/MainContent/UI/W_Dialogue.Talker` (`self.Talker`) (`self.DialWidget`))
  (set `/Game/MainContent/UI/W_Dialogue.Messages` (`self.Messages`) (`self.DialWidget`))
  (`TextBlock.SetText` (`/Game/MainContent/UI/W_Dialogue.FirstName` (`self.DialWidget`)) (`KismetTextLibrary.Conv_StringToText` (`self.FirstName`)))
  (`TextBlock.SetText` (`/Game/MainContent/UI/W_Dialogue.SecondName` (`self.DialWidget`)) (`KismetTextLibrary.Conv_StringToText` (`self.SecondName`)))
  (`/Game/MainContent/UI/W_Dialogue.Click` (`self.DialWidget`))
  (`self.K2_DestroyActor`))

(fn `UserConstructionScript`)