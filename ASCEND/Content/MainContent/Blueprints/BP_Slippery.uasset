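; BP_Slippery is a box-volume actor that makes the ground slippery for the first-person player character inside it.
; When the character's capsule begins overlapping, it caches the movement component's ground friction and walking braking deceleration, then zeroes friction and cuts deceleration to a third.
; When the overlap ends, it restores both cached values from variables stored on the volume.
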(event `self.Box.OnComponentBeginOverlap`
  (params (OverlappedComponent :type "PrimitiveComponent Object Reference") (OtherActor :type "Actor Object Reference") (OtherComp :type "PrimitiveComponent Object Reference") (OtherBodyIndex :type Integer) (bFromSweep :type Boolean) (SweepResult :type "HitResult Structure (by ref)"))
  (bind _ascapsule_collision (cast `CapsuleComponent` OtherComp))
  (bind _asbp_first_person_character (cast `/Game/MainContent/Blueprints/Character/BP_FirstPersonCharacter` (`ActorComponent.GetOwner` _ascapsule_collision)))
  (bind _charactermovement (`Character.CharacterMovement` _asbp_first_person_character))
  (set `self.PreviousGroundFriction` (`CharacterMovementComponent.GroundFriction` _charactermovement))
  (bind _output_get (set `self.PreviousDeceleration` (`CharacterMovementComponent.BrakingDecelerationWalking` _charactermovement)))
  (set `CharacterMovementComponent.BrakingDecelerationWalking` (/ _output_get 3.0) _charactermovement)
  (set `CharacterMovementComponent.GroundFriction` 0.0 _charactermovement))

(event `self.Box.OnComponentEndOverlap`
  (params (OverlappedComponent :type "PrimitiveComponent Object Reference") (OtherActor :type "Actor Object Reference") (OtherComp :type "PrimitiveComponent Object Reference") (OtherBodyIndex :type Integer))
  (bind _ascapsule_collision (cast `CapsuleComponent` OtherComp))
  (bind _asbp_first_person_character (cast `/Game/MainContent/Blueprints/Character/BP_FirstPersonCharacter` (`ActorComponent.GetOwner` _ascapsule_collision)))
  (bind _charactermovement (`Character.CharacterMovement` _asbp_first_person_character))
  (set `CharacterMovementComponent.GroundFriction` (`self.PreviousGroundFriction`) _charactermovement)
  (set `CharacterMovementComponent.BrakingDecelerationWalking` (`self.PreviousDeceleration`) _charactermovement))

(fn `UserConstructionScript`)